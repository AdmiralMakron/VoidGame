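; Checkpoint actor that reports its position relative to the player to the HUD for a map icon.
; Shortly after BeginPlay it attaches a CalcHelper component to the player character's root.
; Each tick it moves that helper to the checkpoint's world location, so its relative location yields the player-local offset, sent to the HUD as 2D.
; GetMapIconData exposes the actor location with a zero icon size.
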(event `self.ReceiveBeginPlay`
  (`KismetSystemLibrary.Delay` 0.2)
  (`SceneComponent.K2_AttachToComponent` (`self.calc_helper`) (`Actor.RootComponent` (`GameplayStatics.GetPlayerCharacter` 0)) "None" "KeepWorld" "KeepWorld" "KeepWorld" true)
  (`self.Update Icon Position`))

(event `self.ReceiveTick`
  (params (DeltaSeconds :type "Float (single-precision)"))
  (`self.Update Icon Position`))

(fn `GetMapIconData`
  (returns (Location :type "Vector Structure") (Icon :type "Texture2D Object Reference") (`Icon Size` :type "Vector2D Structure"))
  (return (`self.K2_GetActorLocation`) null (0.0 0.0)))

(fn `Update Icon Position`
  (`SceneComponent.K2_SetWorldLocation` (`self.calc_helper`) (`self.K2_GetActorLocation`) false false)
  (message `/Game/Null_Undone/MapInterface/BPI_Map.UpdateIconPosition` (`PlayerController.GetHUD` (`GameplayStatics.GetPlayerController` 0)) (`KismetMathLibrary.Conv_VectorToVector2D` (`SceneComponent.RelativeLocation` (`self.calc_helper`)))))

(fn `UserConstructionScript`)