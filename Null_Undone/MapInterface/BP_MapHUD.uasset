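; Map HUD actor that toggles the map widget and feeds player position and heading to the map material.
; Tick writes location and normalized yaw to the MP_Map parameter collection, using the player character as a test stand-in for the Ship.
; Enabling the map creates or reuses WBMap, then spawns viewport icon widgets for every BPI_MapItem actor.
; UpdateIconPosition passes positions to WBMap with X and Y swapped.
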(event `self.ReceiveBeginPlay`)

(event `self.ReceiveTick`
  (params (DeltaSeconds :type "Float (single-precision)"))
  (bind _returnvalue (`GameplayStatics.GetPlayerCharacter` 0))
  (bind _yaw (.yaw (`self.K2_GetActorRotation` _returnvalue)))
  (bind _returnvalue_2 (`GameplayStatics.GetActorOfClass` "/Game/Null_Undone/Ship_Navigation/Ship.Ship_C"))
  (`KismetMaterialLibrary.SetVectorParameterValue` "/Game/Null_Undone/MapInterface/MP_Map.MP_Map" "Ship Location" (`KismetMathLibrary.Conv_VectorToLinearColor` (`self.K2_GetActorLocation` _returnvalue)))
  (`KismetMaterialLibrary.SetScalarParameterValue` "/Game/Null_Undone/MapInterface/MP_Map.MP_Map" "Ship Yaw" (/ (`KismetMathLibrary.SelectFloat` (+ _yaw 360.0) _yaw (< _yaw 0.0)) -360.0)))

(event `/Game/Null_Undone/MapInterface/BPI_Map.UpdateIconPosition`
  (params (Position :type "Vector2D Structure"))
  (bind (_x _y) (`KismetMathLibrary.BreakVector2D` Position))
  (bind _wb_map (`self.WB_Map`)
    (:`then`
      (`/Game/Null_Undone/MapInterface/WBMap.UpdateIconLocation` _wb_map (`KismetMathLibrary.MakeVector2D` _y _x)))
    (:`else`)))

(event `/Game/Null_Undone/MapInterface/BPI_Map.ToggleMap`
  (params (Enabled :type Boolean))
  (if Enabled
    (`self.WB_Map`
      (:`then`
        _)
      (:`else`
        (bind _returnvalue (`|CreateWidget` "/Game/Null_Undone/MapInterface/WBMap.WBMap_C"))
        (set `self.WB_Map` _returnvalue)))
    (`UserWidget.AddToViewport` (`self.WB_Map`) 0)
    (bind _outactors (`GameplayStatics.GetAllActorsWithInterface` "/Game/Null_Undone/MapInterface/BPI_MapItem.BPI_MapItem_C"))
    (for _array_element _outactors
      (bind _returnvalue_2 (`|CreateWidget` "/Game/Null_Undone/MapInterface/WBMap_Icon.WBMap_Icon_C"))
      (bind (_location _icon _icon_size) (message `/Game/Null_Undone/MapInterface/BPI_MapItem.GetMapIconData` _array_element))
      (`/Game/Null_Undone/MapInterface/WBMap_Icon.Initialize Icon` _returnvalue_2 _icon (`KismetMathLibrary.Conv_VectorToVector2D` _location) _icon_size)
      (`UserWidget.AddToViewport` _returnvalue_2 0))
    (else
      (bind _wb_map (`self.WB_Map`)
        (:`then`
          (if (`Widget.IsInViewport` _wb_map)
            (`Widget.RemoveFromParent` _wb_map)))
        (:`else`)))))

(fn `UserConstructionScript`)