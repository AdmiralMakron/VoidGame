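; BP_Item is a pickup actor that the first-person character collects by walking into its sphere.
; On BeginPlay it fills an unset ItemObject from GetDefaultItemObject, which returns nothing here and appears intended for child classes to override.
; Overlap passes ItemObject to the character's inventory component via TryAddItem and destroys the actor only if the add succeeds.
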(event `self.ReceiveBeginPlay`
  (if (not (`KismetSystemLibrary.IsValid` (`self.ItemObject`)))
    (bind _itemobject (`self.GetDefaultItemObject`))
    (set `self.ItemObject` _itemobject)))

(event `self.Sphere.OnComponentBeginOverlap`
  (params (OverlappedComponent :type "PrimitiveComponent Object Reference") (OtherActor :type "Actor Object Reference") (OtherComp :type "PrimitiveComponent Object Reference") (OtherBodyIndex :type Integer) (bFromSweep :type Boolean) (SweepResult :type "HitResult Structure (by ref)"))
  (bind _asbp_first_person_character (cast `/Game/FirstPerson/Blueprints/BP_FirstPersonCharacter` OtherActor))
  (bind _added (`/Game/Inventory/BP_InventoryComponent.TryAddItem` (`/Game/FirstPerson/Blueprints/BP_FirstPersonCharacter.BP_InventoryComponent` _asbp_first_person_character) (`self.ItemObject`)))
  (if _added
    (`self.K2_DestroyActor`)))

(fn `GetDefaultItemObject`
  (returns (ItemObject :type "/Game/Items/BP_Item_Object Object Reference"))
  (return null))

(fn `UserConstructionScript`)