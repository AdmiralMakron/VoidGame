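; Game instance for NullUndone that keeps island layout data so it persists beyond the island actors.
; StoreIslandValues copies each island's transform, seed, type and data into parallel arrays, then clears the actor references.
; Reset empties every array and sets the current island index back to -1.
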(event `self.ReceiveInit`)

(fn `Reset`
  (`KismetArrayLibrary.Array_Clear` (`self.Island Array`))
  (`KismetArrayLibrary.Array_Clear` (`self.Island Locations`))
  (`KismetArrayLibrary.Array_Clear` (`self.Seed Array`))
  (`KismetArrayLibrary.Array_Clear` (`self.Island Types`))
  (`KismetArrayLibrary.Array_Clear` (`self.Island Data`))
  (set `self.CurrIslandIdx` -1))

(fn `Store Island Values`
  (bind _island_array (`self.Island Array`))
  (for _array_element _island_array
    (`KismetArrayLibrary.Array_Add` (`self.Island Locations`) (`Actor.GetTransform` _array_element))
    (`KismetArrayLibrary.Array_Add` (`self.Seed Array`) (`/Game/Islands/BP_Island.Seed` _array_element))
    (`KismetArrayLibrary.Array_Add` (`self.Island Types`) (`/Game/Islands/BP_Island.IslandType` _array_element))
    (`KismetArrayLibrary.Array_Add` (`self.Island Data`) (`/Game/Islands/BP_Island.Data` _array_element)))
  (`KismetArrayLibrary.Array_Clear` _island_array))