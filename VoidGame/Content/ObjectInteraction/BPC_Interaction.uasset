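; Actor component on the first-person character that lets the player interact with objects they look at.
; Each tick it line-traces a short distance from the camera, stores any hit actor implementing BPI_Interaction, and shows its interaction data in the owner's widget.
; When the trace finds nothing interactable, it clears the actor and hides the widget.
; Pressing F sends InteractMessage to the stored actor with the owner as argument.
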(event `self.ReceiveBeginPlay`
  (`KismetSystemLibrary.DelayUntilNextTick`)
  (bind _asbp_first_person_character (cast `/Game/FirstPerson/Blueprints/BP_FirstPersonCharacter` (`self.GetOwner`)))
  (bind _interactionwidget (`/Game/FirstPerson/Blueprints/BP_FirstPersonCharacter.InteractionWidget` _asbp_first_person_character)
    (:`then`
      (set `self.Interaction Widget` _interactionwidget))
    (:`else`)))

(event `self.ReceiveTick`
  (params (DeltaSeconds :type "Float (single-precision)"))
  (`self.InteractionTrace`))

(event `Key|F`
  (params (Key :type "Key Structure"))
  (:`Pressed`
    (bind _interactactor (`self.InteractActor`)
      (:`then`
        (message `/Game/ObjectInteraction/BPI_Interaction.Interact` _interactactor (`self.GetOwner`)))
      (:`else`))))

(fn `InteractionTrace`
  (bind _returnvalue (`GameplayStatics.GetPlayerCameraManager` 0))
  (bind _returnvalue_2 (`Actor.K2_GetActorLocation` _returnvalue))
  (bind (_outhit _returnvalue_3) (`KismetSystemLibrary.LineTraceSingle` :`Start` _returnvalue_2 :`End` (+ _returnvalue_2 (* (`Actor.GetActorForwardVector` _returnvalue) 250.0)) :`TraceChannel` "TraceTypeQuery1" :`TraceColor` (struct :`G` 0.017425 :`B` 1.0 :`A` 1.0)))
  (if _returnvalue_3
    (bind (_bblockinghit _binitialoverlap _time _distance _location _impactpoint _normal _impactnormal _physmat _hitactor) (`GameplayStatics.BreakHitResult` _outhit))
    (if (`KismetSystemLibrary.DoesImplementInterface` _hitactor "/Game/ObjectInteraction/BPI_Interaction.BPI_Interaction_C")
      (bind _output_get (set `self.InteractActor` _hitactor))
      (bind _interacttext (message `/Game/ObjectInteraction/BPI_Interaction.Get_InteractData` _output_get))
      (`/Game/ObjectInteraction/WB_Interaction.Update WBP Interaction` (`self.Interaction Widget`) true _interacttext)
      (else
        (`self.InteractActor` :!label _label
          (:`then`
            (set `self.InteractActor` null)
            (`/Game/ObjectInteraction/WB_Interaction.Update WBP Interaction` (`self.Interaction Widget`) false ""))
          (:`else`))))
    (else
      (goto _label))))