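; BP_R_Tree2 is a tree resource Blueprint that supplies the inventory item produced when the resource is gathered.
; Its GetResourceItemObject function constructs a stackable 2x2 BP_Item_Object, using ResourceBP as the item class and QuantityPerClick as the stack amount.
; The item uses shield icon materials for its normal and rotated views.
; The event graph holds only disabled default events, and the construction script just calls the parent.
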(fn `GetResourceItemObject`
  (returns (Item_Object :type "/Game/Items/BP_Item_Object Object Reference"))
  (bind _returnvalue (`|GenericCreateObject` "/Game/Items/BP_Item_Object.BP_Item_Object_C" (make `IntPoint` 2 2) "/Game/Items/Icons/Placeholders/M_Icon_Shield.M_Icon_Shield" "/Game/Items/Icons/Placeholders/M_Icon_Shield_R.M_Icon_Shield_R" (`self.Resource BP`) false true (`self.Quantity Per Click`)))
  (return _returnvalue))

(fn `UserConstructionScript`
  (`parent.UserConstructionScript`))