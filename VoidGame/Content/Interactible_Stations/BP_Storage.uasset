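; BP_Storage is an interactable storage container, shown as a barrel or chest mesh chosen by ModelType in the construction script.
; When the player enters its box, it shows the transfer grid and copies its inventory into the player's transfer inventory component.
; On exit it copies the items back, clears the transfer component and hides the grid.
; GenerateItems adds wood and stone stacks, but nothing here calls it.
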(event `self.Box.OnComponentBeginOverlap`
  (params (OverlappedComponent :type "PrimitiveComponent Object Reference") (OtherActor :type "Actor Object Reference") (OtherComp :type "PrimitiveComponent Object Reference") (OtherBodyIndex :type Integer) (bFromSweep :type Boolean) (SweepResult :type "HitResult Structure (by ref)"))
  (bind _bp_inventorycomponenttransfer (`/Game/FirstPerson/Blueprints/BP_FirstPersonCharacter.BP_InventoryComponentTransfer` (`self.As BP First Person Character`)))
  (if (== OtherActor (`GameplayStatics.GetPlayerCharacter` 0))
    (bind _asbp_first_person_character (cast `/Game/FirstPerson/Blueprints/BP_FirstPersonCharacter` (`GameplayStatics.GetPlayerCharacter` 0)))
    (bind _output_get (set `self.As BP First Person Character` _asbp_first_person_character))
    (`Widget.SetVisibility` (`/Game/Inventory/WBP_Inventory.WBP_Grid_Inventory_Transfer` (`/Game/FirstPerson/Blueprints/BP_FirstPersonCharacter.InventoryWidget` _output_get)) "Visible")
    (`/Game/Inventory/BP_InventoryComponent.SetItemsArray` _bp_inventorycomponenttransfer (`/Game/Inventory/BP_InventoryComponent.GetItemsArray` (`self.BP_InventoryComponent`)))
    (set `/Game/Inventory/BP_InventoryComponent.IsDirty` true _bp_inventorycomponenttransfer)))

(event `self.Box.OnComponentEndOverlap`
  (params (OverlappedComponent :type "PrimitiveComponent Object Reference") (OtherActor :type "Actor Object Reference") (OtherComp :type "PrimitiveComponent Object Reference") (OtherBodyIndex :type Integer))
  (bind _bp_inventorycomponenttransfer (`/Game/FirstPerson/Blueprints/BP_FirstPersonCharacter.BP_InventoryComponentTransfer` (`self.As BP First Person Character`)))
  (if (== OtherActor (`GameplayStatics.GetPlayerCharacter` 0))
    (`/Game/Inventory/BP_InventoryComponent.SetItemsArray` (`self.BP_InventoryComponent`) (`/Game/Inventory/BP_InventoryComponent.GetItemsArray` _bp_inventorycomponenttransfer))
    (`/Game/Inventory/BP_InventoryComponent.SetItemsArray` _bp_inventorycomponenttransfer (`self.EmptyItems`))
    (set `/Game/Inventory/BP_InventoryComponent.IsDirty` true _bp_inventorycomponenttransfer)
    (`Widget.SetVisibility` (`/Game/Inventory/WBP_Inventory.WBP_Grid_Inventory_Transfer` (`/Game/FirstPerson/Blueprints/BP_FirstPersonCharacter.InventoryWidget` (`self.As BP First Person Character`))) "Hidden")))

(fn `GenerateItems`
  (bind _returnvalue (`|GenericCreateObject` "/Game/Items/BP_Item_Object.BP_Item_Object_C" (make `IntPoint` 2 2) "/Game/Items/Icons/Placeholders/M_Icon_Shield.M_Icon_Shield" "/Game/Items/Icons/Placeholders/M_Icon_Shield_R.M_Icon_Shield_R" "/Game/Items/Materials/BP_Wood.BP_Wood_C" false true 3))
  (`/Game/Inventory/BP_InventoryComponent.TryAddItem` (`self.BP_InventoryComponent`) _returnvalue false 0)
  (bind _returnvalue_2 (`|GenericCreateObject` "/Game/Items/BP_Item_Object.BP_Item_Object_C" (make `IntPoint` 2 2) "/Game/Items/Icons/Placeholders/M_Icon_Shield.M_Icon_Shield" "/Game/Items/Icons/Placeholders/M_Icon_Shield_R.M_Icon_Shield_R" "/Game/Items/Materials/BP_Stone.BP_Stone_C" false true 2))
  (`/Game/Inventory/BP_InventoryComponent.TryAddItem` (`self.BP_InventoryComponent`) _returnvalue_2 false 0))

(fn `UserConstructionScript`
  (switch `/Game/FinalBuild/FinalBuild_BPs/storage_type` (`self.model_type`)
    (:`NewEnumerator0`
      (`StaticMeshComponent.SetStaticMesh` (`self.StaticMesh`) "/Game/FinalBuild/ModelImports/ShipAssets/storage_Barrel.storage_Barrel"))
    (:`NewEnumerator1`
      (`StaticMeshComponent.SetStaticMesh` (`self.StaticMesh`) "/Game/FinalBuild/ModelImports/ShipAssets/storage_Chest.storage_Chest"))))