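; Grid inventory component that stores multi-tile items in a flat Columns by Rows array, with each item referenced in every cell it covers.
; TryAddItem takes the first spot where the item's footprint fits in bounds on empty tiles, retrying once rotated before restoring rotation and failing.
; GetAllItems maps each unique item to its top-left tile.
; Adds and removals set a dirty flag, which Tick turns into one OnInventoryChanged call.
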(event `self.ReceiveBeginPlay`
  (`KismetArrayLibrary.Array_Resize` (`self.Items`) (* (`self.Columns`) (`self.Rows`))))

(event `self.ReceiveTick`
  (params (DeltaSeconds :type "Float (single-precision)"))
  (if (`self.IsDirty`)
    (set `self.IsDirty` false)
    (`self.OnInventoryChanged`)))

(fn `AddItemAt`
  (params (ItemObject :type "/Game/Items/BP_Item_Object Object Reference") (TopLeftIndex :type Integer))
  (bind _tile (`self.ForEachIndex` ItemObject TopLeftIndex)
    (:`LoopBody`
      (`KismetArrayLibrary.Array_Set` (`self.Items`) (`self.TileToIndex` _tile) (`local.ItemObject`)))
    (:`Completed`
      (set `self.IsDirty` true))))

(fn `GetAllItems`
  (returns (AllItems :type "Map of /Game/Items/BP_Item_Object Object Reference to /Game/Inventory/STile Structure"))
  (locals (`AllItems (local)` :type "Map of /Game/Items/BP_Item_Object Object Reference to /Game/Inventory/STile Structure") (`CurrentItemObject (Local)` :type "/Game/Items/BP_Item_Object Object Reference"))
  (for (_array_element _array_index) (`self.Items`)
    (bind _output_get (set `local.CurrentItemObject (Local)` _array_element))
    (`/Engine/EditorBlueprintResources/StandardMacros.IsValid` _output_get
      (:`Is Valid`
        (if (not (`BlueprintMapLibrary.Map_Contains` (`local.AllItems (local)`) _array_element))
          (`BlueprintMapLibrary.Map_Add` (`local.AllItems (local)`) (`local.CurrentItemObject (Local)`) (`self.IndexToTile` _array_index))))))
  (return (`local.AllItems (local)`)))

(fn `GetItemAtIndex`
  (params (Index :type Integer))
  (returns (Valid :type Boolean) (ItemObject :type "/Game/Items/BP_Item_Object Object Reference"))
  (if (`KismetArrayLibrary.Array_IsValidIndex` (`self.Items`) Index)
    (return true (`|GetArrayItem` (`self.Items`) (`local.Index`)))
    (else
      (return false null))))

(fn `IndexToTile`
  (params (Index :type Integer))
  (returns (Tile :type "/Game/Inventory/STile Structure"))
  (bind _columns (`self.Columns`))
  (return (make `/Game/Inventory/STile` (mod Index _columns) (/ Index _columns))))

(fn `IsRoomAvailable`
  (params (ItemObject :type "/Game/Items/BP_Item_Object Object Reference") (TopLeftIndex :type Integer))
  (returns (Result :type Boolean))
  (`|ExecutionSequence`
    (:`then_0`
      (bind _tile (`self.ForEachIndex` (`local.ItemObject`) (`local.TopLeftIndex`))
        (:`LoopBody`
          (`self.IsTileValid` _tile
            (:`true`
              (bind (_valid _itemobject) (`self.GetItemAtIndex` (`self.TileToIndex` _tile)))
              (if _valid
                (if (`KismetSystemLibrary.IsValid` _itemobject)
                  (return false))
                (else
                  (return false))))
            (:`false`
              (return false))))))
    (:`then_1`
      (return true))))

(fn `RemoveItem`
  (params (ItemObject :type "/Game/Items/BP_Item_Object Object Reference"))
  (`/Engine/EditorBlueprintResources/StandardMacros.IsValid` ItemObject
    (:`Is Valid`
      (for (_array_element _array_index) (`self.Items`)
        (if (== _array_element (`local.ItemObject`))
          (`KismetArrayLibrary.Array_Set` (`self.Items`) _array_index)
          (set `self.IsDirty` true))))))

(fn `TileToIndex`
  (params (Tile :type "/Game/Inventory/STile Structure"))
  (returns (index :type Integer))
  (bind (_x _y) (break `/Game/Inventory/STile` Tile))
  (return (+ _x (* _y (`self.Columns`)))))

(fn `TryAddItem`
  (params (ItemObject :type "/Game/Items/BP_Item_Object Object Reference"))
  (returns (Added :type Boolean))
  (`/Engine/EditorBlueprintResources/StandardMacros.IsValid` ItemObject
    (:`Is Valid`
      (for (_ _array_index) (`self.Items`) :!label _label
        (bind _result (`self.IsRoomAvailable` (`local.ItemObject`) _array_index))
        (if _result
          (`self.AddItemAt` (`local.ItemObject`) _array_index)
          (return true)))
      (`|ExecutionSequence`
        (:`then_0`
          (`/Engine/EditorBlueprintResources/StandardMacros.DoOnce` false
            (:`Completed`
              (`/Game/Items/BP_Item_Object.Rotate` (`local.ItemObject`))
              (goto _label))))
        (:`then_1`
          (`/Game/Items/BP_Item_Object.Rotate` (`local.ItemObject`))
          (return false))))))