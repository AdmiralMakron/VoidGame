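; Interactable deck transfer point that teleports the player between the upper and lower decks.
; On BeginPlay its Location setting picks the prompt text and finds actors tagged for the opposite deck, caching the last one's transform as the destination.
; Interact teleports player character 0 to that transform and plays a footstep sound, while GetInteractData supplies the prompt text.
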(event `self.ReceiveBeginPlay`
  (switch `/Game/FinalBuild/FinalBuild_BPs/deck_location` (`self.location`)
    (:`NewEnumerator0`
      (set `self.Interact Text` "Go to Lower Deck")
      (bind _outactors (`GameplayStatics.GetAllActorsWithTag` "lower"))
      (for _array_element _outactors
        (set `self.tp_location` (`self.GetTransform` _array_element))))
    (:`NewEnumerator1`
      (set `self.Interact Text` "Go to Upper Deck")
      (bind _outactors_2 (`GameplayStatics.GetAllActorsWithTag` "upper"))
      (for _array_element_2 _outactors_2
        (set `self.tp_location` (`self.GetTransform` _array_element_2))))))

(event `self.Interact`
  (params (InteractingPlayer :type "Actor Object Reference"))
  ;[1 1 1] Deck Transfer
  (`self.K2_TeleportTo` (`GameplayStatics.GetPlayerCharacter` 0) (.location (`self.tp_location`)) (.rotation (`self.tp_location`)))
  (`GameplayStatics.PlaySound2D` "/Game/Sound_FX/Footsteps_Insert_3.Footsteps_Insert_3" 1.0 1.0 0.0 null null))

(fn `Get_InteractData`
  (returns (InteractText :type String))
  (return (`self.Interact Text`)))

(fn `UserConstructionScript`)