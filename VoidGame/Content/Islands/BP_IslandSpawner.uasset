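; Island spawner that fills the world with randomly typed and seeded BP_Island actors in three distance bands from the origin.
; BeginPlay spawns five islands per band, and Tick adds outer-band islands while the game instance's IslandArray holds fewer than 15.
; Locations combine random X with a square-root-derived positive Y, approximating arcs.
; CreateIsland also adds a map icon when the map widget is in the viewport.
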(event `SpawnIsland1`
  (bind _islandlocation (`self.Get Transform Range` -2700.0 2700.0 3000.0 3100.0))
  (`self.CreateIsland` _islandlocation (`KismetMathLibrary.RandomInteger` 3) (`KismetMathLibrary.RandomInteger` 10000)))

(event `self.ReceiveBeginPlay`
  (bind _counter (`self.Counter`))
  (bind _asbp_null_undone_game_instance (cast `/Game/BP_NullUndone_GameInstance` (`GameplayStatics.GetGameInstance`)))
  ;[1 1 1] Spawns Islands on Startup
  (while (< _counter 5)
    (`self.SpawnIsland1`)
    (`self.SpawnIsland2`)
    (`self.SpawnIsland3`)
    (`/Engine/EditorBlueprintResources/StandardMacros.IncrementInt` _counter)))

(event `SpawnIsland2`
  ;[1 1 1] Spawns islands but in ring 2
  (bind _islandlocation (`self.Get Transform Range` -1800.0 1800.0 2000.0 2100.0))
  (`self.CreateIsland` _islandlocation (`KismetMathLibrary.RandomInteger` 3) (`KismetMathLibrary.RandomInteger` 10000)))

(event `self.ReceiveTick`
  (params (DeltaSeconds :type "Float (single-precision)"))
  (if (< (+ (`KismetArrayLibrary.Array_LastIndex` (`/Game/BP_NullUndone_GameInstance.Island Array` (stale `self.ReceiveBeginPlay` _asbp_null_undone_game_instance))) 1) 15)
    (`self.SpawnIsland1`)))

(event `SpawnIsland3`
  ;[1 1 1] same but in ring 3
  (bind _islandlocation (`self.Get Transform Range` -900.0 900.0 1000.0 1100.0))
  (`self.CreateIsland` _islandlocation (`KismetMathLibrary.RandomInteger` 3) (`KismetMathLibrary.RandomInteger` 10000)))

(fn `CreateIsland`
  (params (`Island Location` :type "Transform Structure") (`Island Type` :type Integer) (Seed :type Integer))
  (bind _returnvalue (`|SpawnActorFromClass` "/Game/Islands/BP_Island.BP_Island_C" `Island Location` "Undefined" "MultiplyWithRoot" null null))
  (set `/Game/Islands/BP_Island.IslandType` `Island Type` _returnvalue)
  (set `/Game/Islands/BP_Island.Seed` Seed _returnvalue)
  (bind _asbp_map_hud (cast `/Game/MapInterface/BP_MapHUD` (`PlayerController.GetHUD` (`GameplayStatics.GetPlayerController` 0))))
  (bind _wb_map (`/Game/MapInterface/BP_MapHUD.WB_Map` _asbp_map_hud)
    (:`then`
      (if (`Widget.IsInViewport` _wb_map)
        (`/Game/MapInterface/BP_MapHUD.CreateIslandIcon` _asbp_map_hud _returnvalue)))
    (:`else`)))

(fn `Get Transform Range`
  (params (MinX :type "Float (double-precision)") (MaxX :type "Float (double-precision)") (MinDistance :type "Float (double-precision)") (MaxDistance :type "Float (double-precision)"))
  (returns (IslandLocation :type "Transform Structure"))
  (bind _returnvalue (`KismetMathLibrary.RandomFloatInRange` MinX MaxX))
  (return (`KismetMathLibrary.MakeTransform` (`KismetMathLibrary.MakeVector` _returnvalue (`KismetMathLibrary.Sqrt` (- (`KismetMathLibrary.RandomFloatInRange` (`KismetMathLibrary.Square` MinDistance) (`KismetMathLibrary.Square` MaxDistance)) (`KismetMathLibrary.Square` _returnvalue)))))))

(fn `SpawnIslands`
  (params (`Island Locations` :type "Array of Transform Structure") (Seed :type "Array of Integer") (`Island Types` :type "Array of Integer"))
  (for (_array_element _array_index) `Island Locations`
    (`self.CreateIsland` _array_element (`|GetArrayItem` Seed _array_index) (`|GetArrayItem` `Island Types`))))

(fn `UserConstructionScript`)