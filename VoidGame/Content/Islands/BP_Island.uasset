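; Island actor that registers in the game instance's IslandArray, takes a material by IslandType, and is destroyed on overlapping BP_BlackHole.
; A looping timer steps it along an atan(X/Y) angle, toward the world origin only for positive Y if unrotated.
; Two distance thresholds from the origin advance MutationLevel, first disabling lighting channels, then swapping material.
; Interact only prints island stats through GenerateIsland; getters expose interact text and icon data.
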(event `self.ReceiveDestroyed`
  (bind _asbp_null_undone_game_instance (cast `/Game/BP_NullUndone_GameInstance` (`GameplayStatics.GetGameInstance`)))
  (`KismetArrayLibrary.Array_RemoveItem` (`/Game/BP_NullUndone_GameInstance.Island Array` _asbp_null_undone_game_instance) self))

(event `self.ReceiveActorBeginOverlap`
  (params (OtherActor :type "Actor Object Reference"))
  (if (== OtherActor (stale `self.ReceiveBeginPlay` _returnvalue))
    (`self.K2_DestroyActor`)))

(event `self.ReceiveBeginPlay`
  (`KismetSystemLibrary.Delay` 0.1)
  (bind _asbp_null_undone_game_instance (cast `/Game/BP_NullUndone_GameInstance` (`GameplayStatics.GetGameInstance`)))
  (`KismetArrayLibrary.Array_Add` (`/Game/BP_NullUndone_GameInstance.Island Array` _asbp_null_undone_game_instance) self)
  (if (== (`self.IslandType`) 0)
    (`PrimitiveComponent.SetMaterial` (`self.StaticMesh`) 0 "/Game/LevelPrototyping/Materials/M_Solid.M_Solid")
    (elif (== (`self.IslandType`) 1)
      (`PrimitiveComponent.SetMaterial` (`self.StaticMesh`) 0 "/Game/LevelPrototyping/Materials/MI_Solid_Blue.MI_Solid_Blue")
      (else
        (`PrimitiveComponent.SetMaterial` (`self.StaticMesh`) 0 "/Game/LevelPrototyping/Materials/M_PrototypeGrid.M_PrototypeGrid"))))
  (bind _returnvalue (`GameplayStatics.GetActorOfClass` "/Game/Islands/BP_BlackHole.BP_BlackHole_C"))
  (`KismetSystemLibrary.K2_SetTimer` null "Update Location" 0.25 true))

(event `Update Location`
  (bind (_returnvalue_x _returnvalue_y) (`KismetMathLibrary.BreakVector` (`self.K2_GetActorLocation`)))
  (bind _returnvalue (`KismetMathLibrary.DegAtan` (/ _returnvalue_x _returnvalue_y)))
  (`self.K2_AddActorLocalTransform` (`KismetMathLibrary.MakeTransform` (`KismetMathLibrary.MakeVector` (* -10.0 (`KismetMathLibrary.DegSin` _returnvalue)) (* -10.0 (`KismetMathLibrary.DegCos` _returnvalue)))))
  (`self.Mutation Check`))

(event `self.ReceiveTick`
  (params (DeltaSeconds :type "Float (single-precision)")))

(event `self.Interact`
  (params (InteractingPlayer :type "Actor Object Reference"))
  ;[1 1 1] put interaction output here
  (bind _harvestresources (`self.HarvestResources`)
    (:`then`
      _)
    (:`else`
      (set `self.HarvestResources` null)))
  (`self.Generate Island` (`self.Seed`) (`self.Mutation Level`) _harvestresources))

(fn `Generate Island`
  (params (Seed :type Integer) (`Mutation Level` :type Integer) (ResourceNodes :type "NiagaraDataInterfaceArrayBool Object Reference"))
  (`KismetSystemLibrary.PrintString` (`KismetStringLibrary.Concat_StrStr` "Seed: " (`KismetStringLibrary.Conv_IntToString` Seed)))
  (`KismetSystemLibrary.PrintString` (`KismetStringLibrary.Concat_StrStr` "Mutation Level:" (`KismetStringLibrary.Conv_IntToString` `Mutation Level`)))
  (`KismetSystemLibrary.PrintString` (`KismetStringLibrary.Concat_StrStr` "Island Type: " (`KismetStringLibrary.Conv_IntToString` (`self.IslandType`)))))

(fn `Get_InteractData`
  (returns (InteractText :type String))
  (return (`self.Interact Text`)))

(fn `GetIslandData`
  (returns (Location :type "Vector Structure") (Icon :type "Texture2D Object Reference") (`Icon Size` :type "Vector2D Structure") (IslandRef :type "/Game/Islands/BP_Island Object Reference"))
  (return (`self.K2_GetActorLocation`) "/Game/MapInterface/planet_icon1.planet_icon1" (20.0 20.0) self))

(fn `Mutate1`
  (set `self.Mutation Level` 1)
  (`PrimitiveComponent.SetLightingChannels` (`self.StaticMesh`) false false false))

(fn `Mutate2`
  (set `self.Mutation Level` 2)
  (`PrimitiveComponent.SetMaterial` (`self.StaticMesh`) 0 "/Game/FPWeapon/Materials/FirstPersonProjectileMaterial.FirstPersonProjectileMaterial"))

(fn `Mutation Check`
  (bind (_returnvalue_x _returnvalue_y) (`KismetMathLibrary.BreakVector` (`self.K2_GetActorLocation`)))
  (bind (_returnvalue_x_2 _returnvalue_y_2) (`KismetMathLibrary.BreakVector` (`self.K2_GetActorLocation`)))
  (if (== (`self.Mutation Level`) 0)
    (if (<= (+ (`KismetMathLibrary.Square` _returnvalue_x) (`KismetMathLibrary.Square` _returnvalue_y)) 4000000.0)
      (`self.Mutate1`))
    (elif (== (`self.Mutation Level`) 1)
      (if (<= (+ (`KismetMathLibrary.Square` _returnvalue_x_2) (`KismetMathLibrary.Square` _returnvalue_y_2)) 1000000.0)
        (`self.Mutate2`)))))

(fn `UserConstructionScript`)