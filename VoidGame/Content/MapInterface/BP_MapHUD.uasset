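; BP_MapHUD is an actor Blueprint that shows and hides the map interface through its ToggleMap event.
; Enabling creates or reuses WBMap, focuses it in Game and UI input, and spawns a WBIsland viewport icon for each BPI_MapItem actor.
; Each icon is initialized from that actor's interface data: texture, 2D world position, size and island reference.
; Disabling removes the map and all island icons, then restores game-only input.
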(event `self.ToggleMap`
  (params (Enabled :type Boolean))
  (bind _returnvalue (`GameplayStatics.GetPlayerController` 0))
  (if Enabled
    (`self.WB_Map`
      (:`then`
        _)
      (:`else`
        (bind _returnvalue_2 (`|CreateWidget` "/Game/MapInterface/WBMap.WBMap_C"))
        (bind _output_get (set `self.WB_Map` _returnvalue_2))))
    (`UserWidget.AddToViewport` _output_get 0)
    (`WidgetBlueprintLibrary.SetInputMode_GameAndUIEx` _returnvalue _output_get)
    (bind _outactors (`GameplayStatics.GetAllActorsWithInterface` "/Game/MapInterface/BPI_MapItem.BPI_MapItem_C"))
    (for _array_element _outactors
      (`self.CreateIslandIcon` _array_element))
    (else
      (bind _wb_map (`self.WB_Map`)
        (:`then`
          (if (`Widget.IsInViewport` _wb_map)
            (`Widget.RemoveFromParent` _wb_map)
            (bind _foundwidgets (`WidgetBlueprintLibrary.GetAllWidgetsOfClass` "/Game/MapInterface/WBIsland.WBIsland_C" false))
            (`Widget.RemoveFromParent` _foundwidgets)
            (`WidgetBlueprintLibrary.SetInputMode_GameOnly` _returnvalue)))
        (:`else`)))))

(fn `CreateIslandIcon`
  (params (IslandRef :type "Actor Object Reference"))
  (bind _returnvalue (`|CreateWidget` "/Game/MapInterface/WBIsland.WBIsland_C"))
  (bind (_location _icon _icon_size _islandref) (message `/Game/MapInterface/BPI_MapItem.GetIslandData` IslandRef))
  (`/Game/MapInterface/WBIsland.Initialize Icon` _returnvalue _icon (`KismetMathLibrary.Conv_VectorToVector2D` _location) _icon_size _islandref)
  (`UserWidget.AddToViewport` _returnvalue 0))

(fn `UserConstructionScript`)